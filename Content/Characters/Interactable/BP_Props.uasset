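; BP_Props is an interactable prop Blueprint that flashes a highlight overlay when something overlaps its Box.
; The Construction Script assigns the configurable MeshAssets static mesh to the Mesh component.
; DoHighlight applies M_Highlight as the overlay material, then clears it after Duration, with a retriggerable delay so repeated calls extend the highlight.
; BeginPlay also applies the overlay without a timer, so it stays until a DoHighlight cycle ends.
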(event OnComponentBeginOverlap(Box)
  (params (OverlappedComponent :type Primitive%20Component%20Object%20Reference) (OtherActor :type Actor%20Object%20Reference) (OtherComp :type Primitive%20Component%20Object%20Reference) (OtherBodyIndex :type Integer) (bFromSweep :type Boolean) (SweepResult :type Hit%20Result%20Structure%20%28by%20ref%29))
  (CallFunction|DoHighlight))

(event Custom|DoHighlight
  (Rendering|Material|SetOverlayMaterial (Variables|Default|GetMesh) "/Game/Materials/M_Highlight.M_Highlight" :!class /Script/Engine.MeshComponent)
  (Utilities|FlowControl|RetriggerableDelay (Variables|Default|GetDuration))
  (Rendering|Material|SetOverlayMaterial (Variables|Default|GetMesh) 0 :!class /Script/Engine.MeshComponent))

(event EventBeginPlay
  (Rendering|Material|SetOverlayMaterial (Variables|Default|GetMesh) "/Game/Materials/M_Highlight.M_Highlight" :!class /Script/Engine.MeshComponent))

(fn ConstructionScript
  (Components|StaticMesh|SetStaticMesh (Variables|Default|GetMesh) (Variables|Default|GetMeshAssets)))