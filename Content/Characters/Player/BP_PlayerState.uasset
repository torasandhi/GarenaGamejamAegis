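; BP_PlayerState is a player state Blueprint that holds tuning values for movement, view and ability cooldowns.
; Interface-style getters return normal and sprint speeds, normal and sprint POV values, and cooldowns for opening the map and showing enemies.
; Each getter passes its variable straight through, and the construction script is empty, so the graphs shown contain no other logic.
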(fn ConstructionScript)

(fn IGetCooldownOpenMap
  (return (Variables|Default|GetCooldownOpenMap)))

(fn IGetCooldownShowEnemy
  (return (Variables|Default|GetCooldownShowEnemy)))

(fn IGetNormalPov
  (return (Variables|Default|GetNormalPov)))

(fn IGetNormalSpeed
  (return (Variables|Default|GetMovementSpeed)))

(fn IGetSprintPov
  (return (Variables|Default|GetSprintPov)))

(fn IGetSprintSpeed
  (return (Variables|Default|GetSprintSpeed)))