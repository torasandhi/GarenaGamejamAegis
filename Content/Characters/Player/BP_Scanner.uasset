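; BP_Scanner is the player's scanner pulse effect, triggered at a given location through the IScan event.
; The event teleports the actor there, restarts two timelines and activates a Niagara effect.
; One timeline scales the actor and drives the sphere material's opacity, collapsing the scale to zero when finished.
; The other animates point light intensity and radius, then deactivates Niagara.
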(event EventIScan
  (params (location :type Vector :default "0, 0, 0"))
  (Transformation|SetActorLocation location false true)
  (Components|Timeline|PlayfromStart (Variables|Default|GetExpandScannr))
  (Components|Timeline|PlayfromStart (Variables|Default|GetScannerLightIntensityTimeline))
  (Components|Activation|Activate (Variables|Default|GetNiagara) false))

(fn ConstructionScript)