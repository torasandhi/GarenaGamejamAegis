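; Player controller that receives Enhanced Input actions and routes them to the player's main character and the HUD.
; On BeginPlay it sets game-only input, caches the BP_MainCharacter pawn and adds the movement, look and mechanic mapping contexts.
; Move, look, sprint, map, show-enemy and interact inputs forward to the character through I-prefixed calls.
; Pause input checks the game's paused state and sends the HUD a pause or unpause message.
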(event Input|EnhancedActionEvents|EnhancedInputActionIA_Move
  (params (ActionValue :type Vector%202D%20Structure) (ElapsedSeconds :type Float%20%28double-precision%29) (TriggeredSeconds :type Float%20%28double-precision%29) (InputAction :type Input%20Action%20Object%20Reference :default "/Game/Input/Actions/IA_Move.IA_Move"))
  (Default|IMove (Variables|Default|GetMain) ActionValue))

(event Input|EnhancedActionEvents|EnhancedInputActionIA_Look
  (params (ActionValue :type Vector%202D%20Structure) (ElapsedSeconds :type Float%20%28double-precision%29) (TriggeredSeconds :type Float%20%28double-precision%29) (InputAction :type Input%20Action%20Object%20Reference :default "/Game/Input/Actions/IA_Look.IA_Look"))
  (Default|ILook (Variables|Default|GetMain) ActionValue))

(event Input|EnhancedActionEvents|EnhancedInputActionIA_OpenMap
  (params (ActionValue :type Boolean) (ElapsedSeconds :type Float%20%28double-precision%29) (TriggeredSeconds :type Float%20%28double-precision%29) (InputAction :type Input%20Action%20Object%20Reference :default "/Game/Input/Actions/IA_OpenMap.IA_OpenMap"))
  (:Started
    (Default|IOpenMap (Variables|Default|GetMain))))

(event Input|EnhancedActionEvents|EnhancedInputActionIA_ShowEnemy
  (params (ActionValue :type Boolean) (ElapsedSeconds :type Float%20%28double-precision%29) (TriggeredSeconds :type Float%20%28double-precision%29) (InputAction :type Input%20Action%20Object%20Reference :default "/Game/Input/Actions/IA_ShowEnemy.IA_ShowEnemy"))
  (:Started
    (Default|IShowEnemy (Variables|Default|GetMain))))

(event Input|EnhancedActionEvents|EnhancedInputActionIA_Sprint
  (params (ActionValue :type Boolean) (ElapsedSeconds :type Float%20%28double-precision%29) (TriggeredSeconds :type Float%20%28double-precision%29) (InputAction :type Input%20Action%20Object%20Reference :default "/Game/Input/Actions/IA_Sprint.IA_Sprint"))
  (:Started
    (Default|ISprint (Variables|Default|GetMain) ActionValue :!label _label))
  (:Completed
    (goto _label)))

(event Input|EnhancedActionEvents|EnhancedInputActionIA_Pause
  (params (ActionValue :type Boolean) (ElapsedSeconds :type Float%20%28double-precision%29) (TriggeredSeconds :type Float%20%28double-precision%29) (InputAction :type Input%20Action%20Object%20Reference :default "/Game/Input/Actions/IA_Pause.IA_Pause"))
  (:Started
    (CallFunction|IsPause)))

(event Input|EnhancedActionEvents|EnhancedInputActionIA_Interact
  (params (ActionValue :type Boolean) (ElapsedSeconds :type Float%20%28double-precision%29) (TriggeredSeconds :type Float%20%28double-precision%29) (InputAction :type Input%20Action%20Object%20Reference :default "/Game/Input/Actions/IA_Interact.IA_Interact"))
  (:Started
    (Default|IInteract (Variables|Default|GetMain))))

(event EventBeginPlay
  (Input|SetInputModeGameOnly self true)
  (CallFunction|FindTarget)
  (CallFunction|BindInput))

(fn ConstructionScript)

(fn FindTarget
  (bind _asbp_main_character (Utilities|Casting|CastToBP_MainCharacter (Game|Player|GetPlayerPawn 0)))
  (Variables|Default|SetMain _asbp_main_character))

(fn BindInput
  (Input|AddMappingContext (PlayerController|LocalPlayerSubsystems|GetEnhancedInputLocalPlayerSubsystem) "/Game/Input/IMC_Movement.IMC_Movement" 0 "(bIgnoreAllPressedKeysUntilRelease=True,bForceImmediately=False,bNotifyUserSettings=False)")
  (Input|AddMappingContext (PlayerController|LocalPlayerSubsystems|GetEnhancedInputLocalPlayerSubsystem) "/Game/Input/IMC_Look.IMC_Look" 0 "(bIgnoreAllPressedKeysUntilRelease=True,bForceImmediately=False,bNotifyUserSettings=False)")
  (Input|AddMappingContext (PlayerController|LocalPlayerSubsystems|GetEnhancedInputLocalPlayerSubsystem) "/Game/Input/IMC_Mechanic.IMC_Mechanic" 0 "(bIgnoreAllPressedKeysUntilRelease=True,bForceImmediately=False,bNotifyUserSettings=False)"))

(fn IsPause
  (bind _returnvalue (HUD|GetHUD))
  (if (Game|IsGamePaused)
    (Class|BPIHUD|IUnpause(Message) _returnvalue)
    (else
      (Class|BPIHUD|IPause(Message) _returnvalue))))