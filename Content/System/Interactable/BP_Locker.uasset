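; Interactable locker with a hinged door that the player can be moved into.
; Interactions alternate through a FlipFlop between opening the door and easing the player to MovePos while the door closes.
; Entering also teleports every enemy from the enemy world subsystem to a random distance in front of the locker.
; The OpenDoor timeline lerps the hinge rotation and toggles CanInteract to block interaction mid-swing.
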(event Custom|MovePlayerInside
  (params (Actor :type Actor%20Object%20Reference))
  (if (not (Variables|Default|GetIsInside))
    (Components|MoveComponentTo (Variables|/Script/Engine.Actor|GetRootComponent Actor) (Transformation|GetWorldLocation (Variables|Default|GetMovePos)) (Variables|/Script/Engine.SceneComponent|GetRelativeRotation (Variables|Default|GetMovePos)) true true 0.5 false)
    (Variables|Default|SetIsInside true)
    (CallFunction|TeleportInfrontOfLocker)))

(event Custom|TeleportInfrontOfLocker
  (bind _returnvalue (Class|EnemyWorldSubsystem|GetAllEnemys (Subsystems|GetEnemyWorldSubsystem)))
  (for _array_element _returnvalue
    (Class|InterfaceEnemy|ISetPosition _array_element (+ (Transformation|GetActorLocation) (* (Transformation|GetActorForwardVector) (Math|Random|RandomFloatinRange 3e+02 4e+02))))))

(event EventIonInteract
  (params (Actor :type Actor%20Object%20Reference))
  (Variables|Default|SetActor Actor)
  (Utilities|FlowControl|FlipFlop
    (:A
      (Components|Timeline|PlayfromStart (Variables|Default|GetOpenDoor)))
    (:B
      (CallFunction|MovePlayerInside (Variables|Default|GetActor))
      (Components|Timeline|ReversefromEnd (Variables|Default|GetOpenDoor))
      (Variables|Default|SetIsInside false))))

(fn ConstructionScript
  (Transformation|SetRelativeRotation (Variables|Default|GetDoorHinge) (Variables|Default|GetRotClosed) false false))

(fn IIsCanInteract
  (return (Variables|Default|GetCanInteract)))