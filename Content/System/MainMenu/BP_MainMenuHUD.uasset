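; BP_MainMenuHUD is the main menu HUD, showing WBP_MainMenu on BeginPlay with UI-only input and a visible cursor.
; Interface-style show and hide events swap between the menu and WBP_Settings, recreating each widget when it is shown.
; IPlayJumpscare only opens Level1, as the level sequence and timed jumpscare widget logic are left disconnected.
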(event EventBeginPlay
  (bind _playerowner (Variables|Default|GetPlayerOwner))
  (bind _returnvalue (UserInterface|CreateWidget "/Game/UserInterface/WBP_MainMenu.WBP_MainMenu_C" (Variables|Default|GetPlayerOwner)))
  (bind _output_get (Variables|Default|SetMainMenuWidget _returnvalue))
  (UserInterface|Viewport|AddtoViewport _output_get 0)
  (Input|SetInputModeUIOnly _playerowner (Variables|Default|GetMainMenuWidget) "DoNotLock" false)
  (Variables|/Script/Engine.PlayerController|SetbShowMouseCursor _playerowner true))

(event EventIPlayJumpscare
  (Game|OpenLevel(byObjectReference) "/Game/Level/Level1.Level1"))

(event EventIShowSettings
  (Utilities|IsValid (Variables|Default|GetSettingsWidget)
    (:Is%20Not%20Valid
      (bind _returnvalue (UserInterface|CreateWidget "/Game/UserInterface/Content/WBP_Settings.WBP_Settings_C" (Variables|Default|GetPlayerOwner)))
      (bind _output_get (Variables|Default|SetSettingsWidget _returnvalue))
      (UserInterface|Viewport|AddtoViewport _output_get 0)
      (Widget|RemovefromParent (Variables|Default|GetMainMenuWidget)))))

(event EventIHideSettings
  (Utilities|IsValid (Variables|Default|GetSettingsWidget)
    (:Is%20Valid
      (bind _returnvalue (UserInterface|CreateWidget "/Game/UserInterface/WBP_MainMenu.WBP_MainMenu_C" (Variables|Default|GetPlayerOwner)))
      (bind _output_get (Variables|Default|SetMainMenuWidget _returnvalue))
      (UserInterface|Viewport|AddtoViewport _output_get 0)
      (Widget|RemovefromParent (Variables|Default|GetSettingsWidget))
      (Variables|Default|SetSettingsWidget 0))))

(fn ConstructionScript)