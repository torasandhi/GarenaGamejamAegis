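; Challenge controller that links a set of interactables to target objects that react when the challenge succeeds or fails.
; On BeginPlay it binds to the success and fail events of every interactable.
; Each success rechecks all interactable conditions and calls ISuccess on every target only when all are true.
; Any fail event calls IFail on every target immediately.
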(event Custom|OnSuccess
  (CallFunction|CheckSuccess))

(event Custom|OnFail
  (for _array_element (Variables|Default|GetTarget)
    (Default|IFail _array_element)))

(event EventBeginPlay
  (for _array_element (Variables|Default|GetInteractable)
    (EventDispatchers|BindEventtoOnSuccess _array_element (EventDispatchers|CreateEvent :!event Custom|OnSuccess))
    (EventDispatchers|BindEventtoOnFail _array_element (EventDispatchers|CreateEvent :!event Custom|OnFail))))

(fn ConstructionScript)

(fn CheckSuccess
  (bind _array_element (Utilities|Array|ForEachLoopwithBreak (Variables|Default|GetInteractable) :!label _label)
    (:LoopBody
      (if (Variables|/Game/System/Challenges/BP_ChallengsActor.BP_ChallengsActor_C|GetCondition _array_element)
        (LocalVariables|SetStatus true)
        (else
          (LocalVariables|SetStatus false)
          (goto _label Break))))
    (:Completed
      (if (LocalVariables|GetStatus)
        (for _array_element_2 (Variables|Default|GetTarget)
          (Default|ISuccess _array_element_2))))))