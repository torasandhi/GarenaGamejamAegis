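; BP_Button is an interactable challenge button that is always available to interact with.
; Interacting sets Condition to true and calls the OnSuccess dispatcher.
; The construction script applies a configurable mesh to the cube and sets the point light's color and attenuation radius.
; A pawn entering the box raises the light's intensity to a fixed value, with no logic to lower it on exit.
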(event OnComponentBeginOverlap(Box)
  (params (OverlappedComponent :type Primitive%20Component%20Object%20Reference) (OtherActor :type Actor%20Object%20Reference) (OtherComp :type Primitive%20Component%20Object%20Reference) (OtherBodyIndex :type Integer) (bFromSweep :type Boolean) (SweepResult :type Hit%20Result%20Structure%20%28by%20ref%29))
  (Utilities|Casting|CastToPawn OtherActor)
  (Rendering|Components|Light|SetIntensity (Variables|Default|GetPointLight) 5e+03))

(event EventBeginPlay
  (|CallParentFunction) ; This node is disabled and will not be called.\nDrag off pins to build functionality.
)

(event Collision|EventActorBeginOverlap
  (params (OtherActor :type Actor%20Object%20Reference))
  (|CallParentFunction OtherActor) ; This node is disabled and will not be called.\nDrag off pins to build functionality.
)

(event EventTick
  (params (DeltaSeconds :type Float%20%28single-precision%29))
  (|CallParentFunction DeltaSeconds) ; This node is disabled and will not be called.\nDrag off pins to build functionality.
)

(event EventIonInteract
  (params (Actor :type Actor%20Object%20Reference))
  (Variables|Default|SetCondition true)
  (Default|CallOnSuccess))

(fn ConstructionScript
  (|CallParentFunction)
  (Components|StaticMesh|SetStaticMesh (Variables|Default|GetCube) (Variables|Default|GetMesh))
  (Rendering|Components|Light|SetLightColor (Variables|Default|GetPointLight) (Math|Conversions|ToLinearColor(Color) (Variables|Default|GetColor)) true)
  (Rendering|Lighting|SetAttenuationRadius (Variables|Default|GetPointLight) (Variables|Default|GetDistance)))

(fn IIsCanInteract
  (return true))